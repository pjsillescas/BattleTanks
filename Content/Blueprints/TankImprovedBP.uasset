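; Player-drivable tank pawn Blueprint that binds input to aiming, firing and movement components.
; On BeginPlay it hands barrel and turret to the aiming component and both tracks to the movement component.
; Aim axes rotate an azimuth gimbal and spring arm, scaled by frame time and a multiplier, to orbit the camera.
; Fire calls the aiming component, while move axes pass forward and turn intents to the movement component.
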(event `self.ReceiveBeginPlay`
  (`TankAimingComponent.Initialize` (`self.TankAimingComponent`) (`self.TankBarrel`) (`self.TankTurret`))
  (`TankMovementComponent.Initialize` (`self.TankMovementComponent`) (`self.LeftTrack`) (`self.RightTrack`)))

(event `InputAxis|AimAzimuth`
  (params (AxisValue :type "Float (single-precision)"))
  ;[1 1 1] Aim Input Binding
  (`SceneComponent.K2_AddLocalRotation` (`self.AzimuthGimbal`) (`KismetMathLibrary.MakeRotator` 0.0 0.0 (* AxisValue (`GameplayStatics.GetWorldDeltaSeconds`) (`self.Multiplier`))) false false))

(event `InputAxis|AimElevation`
  (params (AxisValue :type "Float (single-precision)"))
  ;[1 1 1] Aim Input Binding
  (`SceneComponent.K2_AddLocalRotation` (`self.SpringArm`) (`KismetMathLibrary.MakeRotator` 0.0 (* AxisValue (`GameplayStatics.GetWorldDeltaSeconds`) (`self.Multiplier`))) false false))

(event `InputAction|Fire`
  (params (Key :type "Key Structure"))
  ;[1 1 1] Aim Input Binding
  (:`Pressed`
    (`TankAimingComponent.Fire` (`self.TankAimingComponent`))))

(event `InputAxis|MoveForward`
  (params (AxisValue :type "Float (single-precision)"))
  ;[1 1 1] Movement
  (`TankMovementComponent.IntendMoveForward` (`self.TankMovementComponent`) AxisValue))

(event `InputAxis|MoveRight`
  (params (AxisValue :type "Float (single-precision)"))
  ;[1 1 1] Movement
  (`TankMovementComponent.IntendTurnRight` (`self.TankMovementComponent`) AxisValue))

(fn `UserConstructionScript`)